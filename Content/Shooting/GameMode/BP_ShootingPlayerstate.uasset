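; Player state for the shooting game mode that stores a player's Hp and display name.
; Damage and healing functions clamp Hp between 0 and 100, and a setter assigns the name.
; RepNotify handlers broadcast changes through event dispatchers.
; The Hp handler also prints the value and fires a separate HUD dispatcher only when this state belongs to player controller 0.
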(event EventBeginPlay)

(event EventTick
  (params (DeltaSeconds :type Float%20%28single-precision%29)))

(fn ConstructionScript)

(fn AddDamage
  (params (Damage :type Float%20%28single-precision%29))
  (Variables|Default|SetHp (Math|Float|Clamp(Float) (- (Variables|Default|GetHp) Damage) 0.0 1e+02)))

(fn OnRepHp
  (Development|PrintString (Utilities|String|Append "AddDamage CurHP - " (Utilities|String|ToString(Float) (Variables|Default|GetHp))))
  (Default|CallEventDispatchUpdateHP (Variables|Default|GetHp) 1e+02)
  (if (== (Variables|/Script/Engine.Controller|GetPlayerState (Game|GetPlayerController 0)) self)
    (Default|CallEventDispatcherUpdateHPHUD (Variables|Default|GetHp) 1e+02)))

(fn AddHP
  (params (NewHP :type Float%20%28single-precision%29))
  (Variables|Default|SetHp (Math|Float|Clamp(Float) (+ (Variables|Default|GetHp) NewHP) 0.0 1e+02)))

(fn SetPlayerName
  (params (PlayerName :type String))
  (Variables|Default|SetName PlayerName))

(fn OnRepName
  (Default|CallEventDispatcherChangeName (Variables|Default|GetName)))