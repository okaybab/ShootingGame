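; BP_OverlapActor is a shooting-game actor that disappears when a ShootingCharacter overlaps its static mesh.
; The mesh's begin-overlap event calls OnActorOverlap, which sets IsHidden only on the server authority.
; The IsHidden RepNotify applies the state on server and clients, toggling mesh visibility and switching collision between none and query-and-physics.
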(event OnComponentBeginOverlap(StaticMesh)
  (params (OverlappedComponent :type Primitive%20Component%20Object%20Reference) (OtherActor :type Actor%20Object%20Reference) (OtherComp :type Primitive%20Component%20Object%20Reference) (OtherBodyIndex :type Integer) (bFromSweep :type Boolean) (SweepResult :type Hit%20Result%20Structure%20%28by%20ref%29))
  (Utilities|Casting|CastToShootingCharacter OtherActor)
  (CallFunction|OnActorOverlap OtherActor))

(event Collision|EventActorBeginOverlap
  (params (OtherActor :type Actor%20Object%20Reference)))

(event EventTick
  (params (DeltaSeconds :type Float%20%28single-precision%29)))

(fn ConstructionScript)

(fn OnRepIsHidden
  (bind _ishidden (Variables|Default|GetIsHidden))
  (bind _staticmesh (Variables|Default|GetStaticMesh))
  (Development|SetHiddeninGame (Variables|Default|GetStaticMesh) _ishidden false)
  (if _ishidden
    (Collision|SetCollisionEnabled _staticmesh "NoCollision")
    (else
      (Collision|SetCollisionEnabled _staticmesh "QueryAndPhysics"))))

(fn OnActorOverlap
  (params (otherActor :type Actor%20Object%20Reference))
  (Networking|SwitchHasAuthority
    (:Authority
      (Variables|Default|SetIsHidden true))))