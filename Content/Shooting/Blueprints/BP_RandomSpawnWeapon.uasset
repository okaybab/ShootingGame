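; Spawner Blueprint that periodically drops random, short-lived weapon pickups into the level around player 0.
; BeginPlay caches the DT_Weapon row names and starts a looping one-second timer.
; Each tick of that timer spawns a BP_MachineGun slightly above random navmesh points around the player controller's location, passing a random row name as its weapon name.
; Each spawned gun gets a random lifespan of a few seconds, so it removes itself.
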(event EventBeginPlay
  (bind _outrownames (DataTable|GetDataTableRowNames "/Game/Shooting/Data/DT_Weapon.DT_Weapon"))
  (Variables|Default|SetOut%20Row%20Names _outrownames)
  (Utilities|Time|SetTimerbyFunctionName 0 "RandomSpawnWeapon" 1.0 true))

(event Collision|EventActorBeginOverlap
  (params (OtherActor :type Actor%20Object%20Reference)))

(event EventTick
  (params (DeltaSeconds :type Float%20%28single-precision%29)))

(fn ConstructionScript)

(fn RandomSpawnWeapon
  (bind _returnvalue (Game|GetPlayerController 0))
  (bind _out_row_names (Variables|Default|GetOut%20Row%20Names))
  (bind _returnvalue_2 (Transformation|GetActorLocation _returnvalue))
  (bind _randomlocation (Class|NavigationSystemV1|GetRandomPointinNavigableRadius _returnvalue_2 1e+03 0 0))
  (bind _returnvalue_3 (Game|SpawnActorfromClass "/Game/Shooting/Blueprints/BP_MachineGun.BP_MachineGun_C" (Math|Transform|MakeTransform (Math|Vector|MakeVector (.x _randomlocation) (.y _randomlocation) (+ (.z _randomlocation) 5e+01)) "0, 0, 0" "1,1,1") "Undefined" 0 (Utilities|Array|Get(acopy) _out_row_names (Math|Random|RandomInteger (Utilities|Array|Length _out_row_names))) 0))
  (CallFunction|DestroySpawnWeapon _returnvalue_3))

(fn DestroySpawnWeapon
  (params (NewGun :type BP%20Machine%20Gun%20Object%20Reference))
  (Actor|SetLifeSpan NewGun (Math|Random|RandomFloatinRange 5.0 1e+01)))