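; Weapon actor that characters pick up, fire, reload and drop, configured at BeginPlay from its DT_Weapon row.
; Attach and detach toggle physics and collision on the socketed mesh; trigger and reload play montages, with ammo shown on BP_ShootingHud.
; Separate DoShoot and DoReload handle effects, magazine spawn and refill.
; DoShoot camera-traces only for the local player's pawn, passing hits to Req events for normal or destructible damage.
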(event Custom|ReqApplyDamage
  (params (DamagedActor :type Actor%20Object%20Reference%20%28by%20ref%29) (BaseDamage :type Float%20%28single-precision%29) (EventInstigator :type Controller%20Object%20Reference%20%28by%20ref%29) (DamageCauser :type Actor%20Object%20Reference%20%28by%20ref%29))
  (Game|Damage|ApplyDamage DamagedActor BaseDamage EventInstigator DamageCauser)
  (Development|PrintString (Utilities|String|Append "(Server)ApplyDamage-" (Utilities|GetDisplayName DamagedActor)) false false "(R=1.000000,G=0.000000,B=0.000000,A=1.000000)" 2e+01))

(event Custom|ResDestructible
  (params (Destructible :type Destructible%20Component%20Object%20Reference%20%28by%20ref%29) (DamageAmount :type Float%20%28single-precision%29) (HitLocation :type Vector) (ImpulseDir :type Vector) (ImpulseStrenth :type Float%20%28single-precision%29))
  (Class|DestructibleComponent|ApplyDamage Destructible DamageAmount HitLocation ImpulseDir ImpulseStrenth))

(event Custom|ReqDestructible
  (params (Destructible :type Destructible%20Component%20Object%20Reference%20%28by%20ref%29) (DamageAmount :type Float%20%28single-precision%29) (HitLocation :type Vector) (ImpulseDir :type Vector) (ImpulseStrenth :type Float%20%28single-precision%29))
  (CallFunction|ResDestructible Destructible DamageAmount HitLocation ImpulseDir ImpulseStrenth))

(event EventBeginPlay
  (CallFunction|Initialize))

(event Collision|EventActorBeginOverlap
  (params (OtherActor :type Actor%20Object%20Reference)))

(event EventTick
  (params (DeltaSeconds :type Float%20%28single-precision%29)))

(fn ConstructionScript)

(fn PlayShootMontage
  (bind _ownchar (Variables|Default|GetOwnChar))
  (bind _weapondata (Variables|Default|GetWeaponData))
  (bind (_staticmesh _socketname _shootsound _reloadsound _ammo _shootmontage _shootmontageplayrate) (Utilities|Struct|BreakST_Weapon _weapondata))
  (if (CallFunction|CheckShootable)
    (Utilities|IsValid _ownchar
      (:Is%20Valid
        (Animation|Montage|MontagePlay (Components|SkeletalMesh|GetAnimInstance (Variables|/Script/Engine.Character|GetMesh _ownchar)) _shootmontage _shootmontageplayrate "MontageLength" 0.0 true)
        (bind _result (Math|Integer|DecrementInt (Variables|Default|GetCurAmmo))
          (:%20%20
            (Development|PrintString (Utilities|String|ToString(Integer) _result) false false)
            (bind _asbp_shooting_hud (Utilities|Casting|CastToBP_ShootingHud (HUD|GetHUD (Game|GetPlayerController 0))))
            (Default|SetAmmoText _asbp_shooting_hud _result)))))))

(fn CheckShootable
  (Utilities|IsValid (Variables|Default|GetOwnChar)
    (:Is%20Valid
      (if (> (Variables|Default|GetCurAmmo) 0)
        (return true)
        (else
          (return false))))
    (:Is%20Not%20Valid
      (return false))))

(fn PlayReloadMontage
  (bind _ownchar (Variables|Default|GetOwnChar))
  (bind _weapondata (Variables|Default|GetWeaponData))
  (bind (_staticmesh _socketname _shootsound _reloadsound _ammo _shootmontage _shootmontageplayrate _reloadmontage _reloadmontageplayrate) (Utilities|Struct|BreakST_Weapon _weapondata))
  (Utilities|IsValid _ownchar
    (:Is%20Valid
      (Animation|PlayAnimMontage _ownchar _reloadmontage _reloadmontageplayrate "None"))))

(fn Initialize
  (bind _returnvalue (Utilities|GetDataTableRow "/Game/Shooting/Data/DT_Weapon.DT_Weapon" (Variables|Default|GetWeaoonName))
    (:then
      (bind _output_get (Variables|Default|SetWeaponData _returnvalue))
      (Components|StaticMesh|SetStaticMesh (Variables|Default|GetStaticMesh) (.StaticMesh (Utilities|Struct|BreakST_Weapon _output_get)))
      (Variables|Default|SetSocket%20Name (.SocketName (Utilities|Struct|BreakST_Weapon _output_get)))
      (Audio|Components|Audio|SetSound (Variables|Default|GetAudio_shoot) (.ShootSound (Utilities|Struct|BreakST_Weapon _output_get)))
      (Variables|Default|SetCurAmmo (.Ammo (Utilities|Struct|BreakST_Weapon _output_get))))))

(fn FindActorHP)

(fn AttachtoChar
  (params (Character :type Character%20Object%20Reference))
  (bind _staticmesh (Variables|Default|GetStaticMesh))
  (bind _output_get (Variables|Default|SetOwnChar Character))
  (Utilities|Time|SetTimerbyFunctionName 0 "FindActorHP" 0.01 true)
  (bind _asbp_shooting_hud (Utilities|Casting|CastToBP_ShootingHud (HUD|GetHUD (Game|GetPlayerController 0))))
  (Default|SetAmmoText _asbp_shooting_hud (Variables|Default|GetCurAmmo))
  (Default|SetMaxAmmoText _asbp_shooting_hud (.Ammo (Utilities|Struct|BreakST_Weapon (Variables|Default|GetWeaponData))))
  (Physics|SetSimulatePhysics _staticmesh false)
  (Collision|SetCollisionEnabled _staticmesh "NoCollision")
  (bind _returnvalue (Transformation|AttachComponentToComponent _staticmesh (Variables|/Script/Engine.Character|GetMesh _output_get) (Variables|Default|GetSocket%20Name) "SnapToTarget" "SnapToTarget" "KeepWorld" true))
  (return _returnvalue self))

(fn DetachtoChar
  (params (Character :type Character%20Object%20Reference))
  (bind _staticmesh (Variables|Default|GetStaticMesh))
  (Variables|Default|SetOwnChar 0)
  (Utilities|Time|ClearTimerbyFunctionName 0 "FindActorHP")
  (Collision|SetCollisionEnabled _staticmesh "QueryAndPhysics")
  (Physics|SetSimulatePhysics _staticmesh true)
  (Transformation|DetachFromComponent _staticmesh "KeepWorld" "KeepWorld" "KeepWorld" true)
  (return true))

(fn DoReload
  (params (Character :type Character%20Object%20Reference))
  (Audio|Components|Audio|Play (Variables|Default|GetAudio_reload) 0.0)
  (Game|SpawnActorfromClass "/Game/Shooting/Blueprints/SM_KA47_Mag_Empty.SM_KA47_Mag_Empty_C" (Math|Transform|MakeTransform (Transformation|GetSocketLocation (Variables|Default|GetStaticMesh) "Boolet") "0, 0, 0" "1,1,1") "Undefined" 0 0)
  (bind _output_get (Variables|Default|SetCurAmmo (.Ammo (Utilities|Struct|BreakST_Weapon (Variables|Default|GetWeaponData)))))
  (bind _asbp_shooting_hud (Utilities|Casting|CastToBP_ShootingHud (HUD|GetHUD (Game|GetPlayerController 0))))
  (Default|SetAmmoText _asbp_shooting_hud _output_get)
  (return false))

(fn DoShoot
  (params (Character :type Character%20Object%20Reference))
  (bind _returnvalue (Game|GetPlayerCameraManager 0))
  (bind _returnvalue_2 (Transformation|GetActorLocation _returnvalue))
  (Audio|Components|Audio|Play (Variables|Default|GetAudio_shoot) 0.0)
  (Effects|SpawnEmitteratLocation "/Game/StarterContent/Particles/P_Explosion.P_Explosion" (Transformation|GetSocketLocation (Variables|Default|GetStaticMesh) "Muzzle") "0, 0, 0" "0.100000,0.100000,0.100000")
  ;[1 1 1] 소유한 클라이언트에서 히트 체크
  (if (== (Variables|Default|GetOwnChar) (Game|Player|GetPlayerPawn 0))
    (bind (_outhit _returnvalue_3) (Collision|LineTraceForObjects (+ _returnvalue_2 (* (Transformation|GetActorForwardVector _returnvalue) 3e+02)) (+ _returnvalue_2 (* (Transformation|GetActorForwardVector _returnvalue) 1e+04)) (Utilities|Array|MakeArray "ObjectTypeQuery1" "ObjectTypeQuery2" "ObjectTypeQuery3" "ObjectTypeQuery4" "ObjectTypeQuery6") false 0 "ForDuration" true "(R=1.000000,G=0.000000,B=0.000000,A=1.000000)" "(R=0.000000,G=1.000000,B=0.000000,A=1.000000)" 1.0))
    (if _returnvalue_3
      (bind _asdestructible_component (Utilities|Casting|CastToDestructibleComponent (.HitComponent (Collision|BreakHitResult _outhit)))
        (:then
          (CallFunction|ReqDestructible _asdestructible_component 1e+02 (.ImpactPoint (Collision|BreakHitResult _outhit)) (Transformation|GetActorForwardVector (Game|GetPlayerCameraManager 0)) 1e+04)
          (return true))
        (:CastFailed
          (Development|PrintString "(Client) ReqApplyDamage" false false "(R=0.000000,G=0.660000,B=1.000000,A=1.000000)" 2e+01)
          (CallFunction|ReqApplyDamage (.HitActor (Collision|BreakHitResult _outhit)) 1e+01 (Pawn|GetController (Variables|Default|GetOwnChar)) self)
          (return true))))))

(fn PullTrigger
  (params (Character :type Character%20Object%20Reference))
  (CallFunction|PlayShootMontage)
  (return true))

(fn ReleaseTrigger
  (params (Character :type Character%20Object%20Reference))
  (return false))

(fn ReloadAmmo
  (params (Character :type Character%20Object%20Reference))
  (CallFunction|PlayReloadMontage)
  (return false))