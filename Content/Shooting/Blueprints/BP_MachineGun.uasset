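; BP_MachineGun is an automatic weapon Blueprint that keeps firing while the trigger is held.
; PullTrigger fires once and starts a looping timer on PlayShootMontage, which ReleaseTrigger clears.
; Each shot passes the parent's CheckShootable, plays a sped-up rifle montage on the owning character, decrements ammo, prints it and updates the shooting HUD.
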(event EventBeginPlay
  (|CallParentFunction) ; 지금 이 노드는 비활성 상태입니다. \n핀을 끌어서 다른 노드를 연결하면 활성화됩니다.
)

(event Collision|EventActorBeginOverlap
  (params (OtherActor :type Actor%20Object%20Reference))
  (|CallParentFunction OtherActor) ; 지금 이 노드는 비활성 상태입니다. \n핀을 끌어서 다른 노드를 연결하면 활성화됩니다.
)

(event EventTick
  (params (DeltaSeconds :type Float%20%28single-precision%29))
  (|CallParentFunction DeltaSeconds) ; 지금 이 노드는 비활성 상태입니다. \n핀을 끌어서 다른 노드를 연결하면 활성화됩니다.
)

(fn ConstructionScript
  (|CallParentFunction))

(fn PullTrigger
  (params (Character :type Character%20Object%20Reference))
  (CallFunction|PlayShootMontage)
  (Utilities|Time|SetTimerbyFunctionName 0 "PlayShootMontage" 0.1 true)
  (return true))

(fn ReleaseTrigger
  (params (Character :type Character%20Object%20Reference))
  (Utilities|Time|ClearTimerbyFunctionName 0 "PlayShootMontage")
  (return false))

(fn PlayShootMontage
  (bind _ownchar (Variables|Default|GetOwnChar))
  (if (CallFunction|CheckShootable)
    (Utilities|IsValid _ownchar
      (:Is%20Valid
        (Animation|Montage|MontagePlay (Components|SkeletalMesh|GetAnimInstance (Variables|/Script/Engine.Character|GetMesh _ownchar)) "/Game/Mannequin/Animations/InPlace/Rifle_ShootOnce_Montage.Rifle_ShootOnce_Montage" 1.5 "MontageLength" 0.0 true)
        (bind _result (Math|Integer|DecrementInt (Variables|Default|GetAmmo))
          (:%20%20
            (Development|PrintString (Utilities|String|ToString(Integer) _result))
            (bind _asbp_shooting_hud (Utilities|Casting|CastToBP_ShootingHUd (HUD|GetHUD (Game|GetPlayerController 0))))
            (Default|SetAmmoText _asbp_shooting_hud _result)))))))

(fn CheckShootable
  (return (|CallParentFunction)))